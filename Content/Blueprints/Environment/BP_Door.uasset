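; BP_Door is an environment door Blueprint that tracks whether the door is open or closed.
; On BeginPlay it binds its open and close events to the OpenDoor and CloseDoor event dispatchers.
; Those events call functions that check the current state and flip the IsDoorOpen boolean only when it differs.
; The graphs change state only, with no movement, animation or sound.
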(event Custom|Open%20Door
  (CallFunction|FOpenDoor))

(event Custom|Close%20Door
  (CallFunction|FCloseDoor))

(event EventBeginPlay
  (EventDispatchers|BindEventtoOpenDoor (delegate Custom|Open%20Door))
  (EventDispatchers|BindEventtoCloseDoor (delegate Custom|Close%20Door)))

(fn ConstructionScript)

(fn FOpenDoor
  (bind _isdooropen (CallFunction|FIsDoorOpen))
  (if (not _isdooropen)
    (Variables|Default|SetIsDoorOpen true)))

(fn FCloseDoor
  (bind _isdooropen (CallFunction|FIsDoorOpen))
  (if _isdooropen
    (Variables|Default|SetIsDoorOpen false)))

(fn FIsDoorOpen
  (if (Variables|Default|GetIsDoorOpen)
    (return true)
    (else
      (return false))))