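; Fire extinguisher tool Blueprint that, as written, only simulates a draining battery life.
; Tick passes world time to FExpendBatteryLife, which acts whenever the rounded seconds exceed the stored SecondsPassed.
; While battery remains, it subtracts total seconds times a multiplier, so drain accelerates over time, and prints the level as a percentage.
; The value is not clamped at zero, and no extinguishing logic is present.
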(event EventTick
  (params (DeltaSeconds :type Float%20%28single-precision%29))
  (CallFunction|FExpendBatteryLife (Utilities|Time|GetTimeSeconds)))

(fn ConstructionScript)

(fn FExpendBatteryLife
  (params (Seconds :type Float%20%28single-precision%29))
  (bind _returnvalue (Math|Float|Round Seconds))
  (if (> _returnvalue (LocalVariables|GetSecondsPassed))
    (LocalVariables|SetSecondsPassed _returnvalue)
    (if (> (Variables|Default|GetBatteryLife) 0.0)
      (bind _output_get (Variables|Default|SetBatteryLife (- (Variables|Default|GetBatteryLife) (* (LocalVariables|GetSecondsPassed) (Variables|Default|GetBatteryExpenditureMultiplier)))))
      (Development|PrintString (Utilities|String|Append "Battery is at:" (Utilities|String|ToString(Float) _output_get) "%")))))