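; SSController is a controller Blueprint that relays player input to the level's BaseCharacter.
; On BeginPlay it caches the first BaseCharacter found by GetAllActorsOfClass as CharacterRef.
; The X and Y axis inputs and the release of Interact call matching pass-through events on that reference, leaving the response to the character.
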(event EventBeginPlay
  (bind _outactors (Actor|GetAllActorsOfClass "/Game/Blueprints/CharacterStuff/BaseCharacter.BaseCharacter_C"))
  (Variables|Default|SetCharacterRef (Utilities|Array|Get(acopy) _outactors)))

(event Input|ActionEvents|InputActionInteract
  (params (Key :type Key%20Structure :default "None"))
  (:Released
    (Default|InteractPassEvent (Variables|Default|GetCharacterRef))))

(event Input|AxisEvents|InputAxisY-Axis
  (params (AxisValue :type Float%20%28single-precision%29))
  (Default|Y-AxisPassEvent (Variables|Default|GetCharacterRef) AxisValue))

(event Input|AxisEvents|InputAxisX-AxisMap
  (params (AxisValue :type Float%20%28single-precision%29))
  (Default|X-AxisPassEvent (Variables|Default|GetCharacterRef) AxisValue))

(event Input|KeyboardEvents|T
  (params (Key :type Key%20Structure :default "None")))

(fn ConstructionScript)