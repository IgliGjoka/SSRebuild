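; Base character Blueprint with pass-through events for movement and interaction, plus a getter that returns itself.
; The X and Y axis events share one CharacterMovement AddInputVector call in world space, leaving control-yaw direction vectors unconnected.
; Interact fires a debug-drawn Visibility line trace forward from the CastArrowTarget component, but nothing uses the hit result yet.
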(event Custom|InteractPassEvent
  (bind _cast_arrow_target (Variables|Default|GetCast%20Arrow%20Target))
  (bind _returnvalue (Transformation|GetWorldLocation _cast_arrow_target))
  (Collision|LineTraceByChannel _returnvalue (+ _returnvalue (* (Math|Vector|GetForwardVector (Transformation|GetWorldRotation _cast_arrow_target)) 3e+02)) "TraceTypeQuery1" false 0 "ForDuration"))

(event Custom|Y-AxisPassEvent
  (params (Axis :type Float%20%28single-precision%29))
  ;[1 1 1] testGIT
  (Class|PawnMovementComponent|AddInputVector (Variables|Character|GetCharacterMovement) (Math|Vector|MakeVector (stale Custom|X-AxisPassEvent Axis) Axis 0.0) false))

(event Custom|X-AxisPassEvent
  (params (Axis :type Float%20%28single-precision%29))
  ;[1 1 1] testGIT
  (Class|PawnMovementComponent|AddInputVector (Variables|Character|GetCharacterMovement) (Math|Vector|MakeVector Axis (stale Custom|Y-AxisPassEvent Axis) 0.0) false))

(event EventBeginPlay)

(fn ConstructionScript)

(fn PlayerCharacterRefrenceGetter
  (return self))