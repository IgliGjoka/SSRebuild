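; CameraBP is a follow-camera actor that tracks the first BaseCharacter found in the level.
; On BeginPlay it finds and caches that character.
; Each Tick it moves itself to the character's position, offset back along world X by XMin and raised by ZMin, matching Y exactly.
; The height is clamped so it never drops below ZMin, and the movement has no smoothing or rotation update.
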(event EventTick
  (params (DeltaSeconds :type Float%20%28single-precision%29))
  (bind _zmin (Variables|Default|GetZMin))
  (bind _character_array (Variables|Default|GetCharacter%20Array))
  (bind _returnvalue (Transformation|GetActorLocation _character_array))
  (Transformation|SetActorLocation (Math|Vector|MakeVector (- (.x _returnvalue) (Variables|Default|GetXMin)) (.y _returnvalue) (Math|Float|Clamp(Float) (+ (.z _returnvalue) _zmin) _zmin 1e+05)) false false))

(event EventBeginPlay
  (bind _outactors (Actor|GetAllActorsOfClass "/Game/Blueprints/CharacterStuff/BaseCharacter.BaseCharacter_C"))
  (Variables|Default|SetCharacter%20Array (Utilities|Array|Get(acopy) _outactors)))

(fn ConstructionScript)