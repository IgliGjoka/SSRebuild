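; Solar Sailor game mode that periodically sets off random hazards in the level.
; BeginPlay gathers all CoreHazardClass actors and starts a looping five-second timer.
; Each tick of that timer rebuilds the candidate list from hazards in one particular HazardState and calls TriggerRecieved on a random entry.
; When no hazard qualifies, the timer is cleared, and nothing in this graph restarts it.
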(event Custom|Hazard%20Trigger
  (CallFunction|ActivateRandomHazard))

(event Custom|Begin%20Trigger%20Activation%20Timer
  (bind _returnvalue (Utilities|Time|SetTimerbyEvent (delegate Custom|Hazard%20Trigger) 5.0 true))
  (Variables|Default|SetHazard%20Trigger%20Timer _returnvalue))

(event EventBeginPlay
  (bind _outactors (Actor|GetAllActorsOfClass "/Game/Blueprints/NathanielDunbabin/HazardAssets/CoreHazardClass.CoreHazardClass_C"))
  (for _array_element _outactors
    (Utilities|Array|AddUnique (Variables|Default|GetUnsafe%20Hazard%20Refrences) _array_element))
  (Variables|Default|SetHazard%20Max%20Index%20Range (- (Utilities|Array|Length (Variables|Default|GetUnsafe%20Hazard%20Refrences)) 1))
  (CallFunction|BeginTriggerActivationTimer))

(event EventTick
  (params (DeltaSeconds :type Float%20%28single-precision%29)))

(fn ConstructionScript)

(fn ActivateRandomHazard
  (bind _unsafe_hazard_refrences (Variables|Default|GetUnsafe%20Hazard%20Refrences))
  (bind _returnvalue (Utilities|Array|Length _unsafe_hazard_refrences))
  (bind _returnvalue_2 (- _returnvalue 1))
  (bind _returnvalue_3 (Math|Random|RandomIntegerinRange 0 _returnvalue_2))
  ;[1 1 1] Find a random hazard that is currently susceptible to activation and activate it.
  (Utilities|Array|Clear (Variables|Default|GetUnsafe%20Hazard%20Refrences))
  (bind _outactors (Actor|GetAllActorsOfClass "/Game/Blueprints/NathanielDunbabin/HazardAssets/CoreHazardClass.CoreHazardClass_C"))
  (for _array_element _outactors
    (if (Utilities|Enum|Equal(Enum) (Variables|/Game/Blueprints/NathanielDunbabin/HazardAssets/CoreHazardClass.CoreHazardClass_C|GetHazard%20State _array_element) "NewEnumerator1")
      (Utilities|Array|AddUnique (Variables|Default|GetUnsafe%20Hazard%20Refrences) _array_element)))
  (if (Utilities|Array|IsValidIndex (Variables|Default|GetUnsafe%20Hazard%20Refrences) _returnvalue_3)
    (Default|TriggerRecieved (Utilities|Array|Get(acopy) (Variables|Default|GetUnsafe%20Hazard%20Refrences) _returnvalue_3))
    (else
      (Utilities|Time|ClearandInvalidateTimerbyHandle (Variables|Default|GetHazard%20Trigger%20Timer))))
  (return))

(fn GetSolarSailorObjectRefrence
  (return self))