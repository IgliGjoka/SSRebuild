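; Tool counter actor that displays a tool as a child actor, apparently intended to store the player's tool.
; Construction script sets the child actor class, and a timeline started on BeginPlay bobs and spins it.
; Platform overlap with BaseCharacter opens or closes a gate for the interaction event.
; Storage is unfinished: the ToolStored branch is empty and GetAndStorePlayerTool only clears the held class.
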(event OnComponentBeginOverlap(ToolCounterPlatform)
  (params (OverlappedComponent :type Primitive%20Component%20Object%20Reference) (OtherActor :type Actor%20Object%20Reference) (OtherComp :type Primitive%20Component%20Object%20Reference) (OtherBodyIndex :type Integer) (bFromSweep :type Boolean) (SweepResult :type Hit%20Result%20Structure%20%28by%20ref%29))
  (if (== OtherActor "/Game/Blueprints/CharacterStuff/BaseCharacter.BaseCharacter")
    (Utilities|FlowControl|Gate true) ; enters at Open
  ))

(event OnComponentEndOverlap(ToolCounterPlatform)
  (params (OverlappedComponent :type Primitive%20Component%20Object%20Reference) (OtherActor :type Actor%20Object%20Reference) (OtherComp :type Primitive%20Component%20Object%20Reference) (OtherBodyIndex :type Integer))
  (if (== OtherActor "/Game/Blueprints/CharacterStuff/BaseCharacter.BaseCharacter")
    (Utilities|FlowControl|Gate true) ; enters at Close
  ))

(event Custom|Player%20Interaction%20Event
  (Utilities|FlowControl|Gate true
    (:Exit
      (if (Variables|Default|GetTool%20Stored?)
        _))))

(event EventBeginPlay
  (bind _tool_bob (Timeline|Tool%20movement Play)
    (:Update
      (Transformation|SetRelativeLocation (Variables|Default|GetTooltohold) _tool_bob false false)
      (Transformation|AddRelativeRotation (Variables|Default|GetTooltohold) (Math|Rotator|MakeRotator 0.0 0.0 0.5) false false))))

(event Collision|EventActorBeginOverlap
  (params (OtherActor :type Actor%20Object%20Reference)))

(event EventTick
  (params (DeltaSeconds :type Float%20%28single-precision%29)))

(fn ConstructionScript
  (ChildActorComponent|SetChildActorClass (Variables|Default|GetTooltohold) (Variables|Default|GetTool%20This%20counter%20holds)))

(fn GetandStorePlayerTool
  (params (Actor%20Ref :type Actor%20Object%20Reference))
  ;[1 1 1] This talks to the player pawn, and removes their currently selected tool, setting the 'Tooltohold' child actor to that tool
  (Variables|Default|SetTool%20This%20counter%20holds 0))